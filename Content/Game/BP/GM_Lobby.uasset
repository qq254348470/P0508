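; Lobby game mode that tracks joining players and shares the player info list and selected level name with them.
; On login it stores the controller, spawns and possesses a BP_Lobby pawn at the first PlayerStart found, then has Controller_Lobby initialise and create its UI.
; The level name comes from GM_Instance at BeginPlay, and an update event pushes it with the accumulated player info to every lobby controller.
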(event Custom|SpawnPawn_CS
  (params (PC :type Controller%20Object%20Reference))
  (bind _returnvalue (Pawn|GetControlledPawn PC))
  (Utilities|IsValid _returnvalue
    (:Is%20Valid
      (Actor|DestroyActor _returnvalue))
    (:Is%20Not%20Valid
      _))
  (bind _outactors (Actor|GetAllActorsOfClass "/Script/Engine.PlayerStart"))
  (bind _returnvalue_2 (Game|SpawnActorfromClass "/Game/Game/BP/BP_Lobby.BP_Lobby_C" (Transformation|GetActorTransform (Utilities|Array|Get(acopy) _outactors)) "AdjustIfPossibleButAlwaysSpawn" 0 0))
  (Pawn|Possess PC _returnvalue_2))

(event Custom|UpdateInfo_CS
  (for _array_element (Variables|Default|GetPlayerList)
    (bind _ascontroller_lobby (Utilities|Casting|CastToController_Lobby _array_element))
    (Default|UpdateSelfCS _ascontroller_lobby (Variables|Default|GetPlayerInfo) (Variables|Default|GetLevelName))))

(event Custom|AddPlayerInfo_CS
  (params (NewItem :type Struct%20Player%20Info%20Structure%20%28by%20ref%29))
  (Utilities|Array|Add (Variables|Default|GetPlayerInfo) NewItem))

(event EventBeginPlay
  (bind _asgm_instance (Utilities|Casting|CastToGM_Instance (Game|GetGameInstance)))
  (Variables|Default|SetLevelName (Variables|/Game/Start/BP/GM_Instance.GM_Instance_C|GetLevelName _asgm_instance))
  (CallFunction|UpdateInfoCS))

(event EventTick
  (params (DeltaSeconds :type Float%20%28single-precision%29)))

(event EventPostLogin
  (params (NewPlayer :type Player%20Controller%20Object%20Reference))
  (Utilities|Array|Add (Variables|Default|GetPlayerList) NewPlayer)
  (CallFunction|SpawnPawnCS NewPlayer)
  (bind _ascontroller_lobby (Utilities|Casting|CastToController_Lobby NewPlayer))
  (Default|InitCS _ascontroller_lobby)
  (Default|CreateUMGCS _ascontroller_lobby))

(fn ConstructionScript)

(fn GetAllPlayerInfoCS
  (for _array_element (Variables|Default|GetPlayerList)
    (bind _ascontroller_lobby (Utilities|Casting|CastToController_Lobby _array_element))
    (Utilities|Array|Add (LocalVariables|GetPlayerInfo11) (Variables|/Game/Game/BP/Controller_Lobby.Controller_Lobby_C|GetPlayerInfo _ascontroller_lobby)))
  (return (LocalVariables|GetPlayerInfo11)))